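; Damage puddle actor that hurts player-controlled characters inside its area of effect and destroys itself after a fixed lifetime.
; Area enter and exit events filter for player-controlled pawns, then start or stop the damage.
; Entering deals an immediate hit and starts a looping timer that repeatedly calls TakeDamage on the ThirdPersonCharacter.
; A single stored timer handle is cleared on exit.
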(event Custom|Start%20Damage
  (params (Affected%20Pawn :type Pawn%20Object%20Reference))
  (CallFunction|InflictDamage)
  (bind _returnvalue (Utilities|Time|SetTimerbyEvent (delegate Custom|Inflict%20Damage) 0.2 true)))

(event Custom|Inflict%20Damage
  (bind _asthird_person_character (Utilities|Casting|CastToThirdPersonCharacter (stale Custom|Start%20Damage Affected%20Pawn)))
  (Default|TakeDamage _asthird_person_character 2.0))

(event Custom|Stop%20Damage
  (Utilities|Time|ClearandInvalidateTimerbyHandle (stale Custom|Start%20Damage _returnvalue)))

(event EventBeginPlay
  (|CallParentFunction)
  (Utilities|FlowControl|Delay 2e+01)
  (Actor|DestroyActor))

(event Collision|EventActorBeginOverlap
  (params (OtherActor :type Actor%20Object%20Reference))
  (|CallParentFunction OtherActor) ; This node is disabled and will not be called.\nDrag off pins to build functionality.
)

(event EventTick
  (params (DeltaSeconds :type Float%20%28single-precision%29))
  (|CallParentFunction DeltaSeconds) ; This node is disabled and will not be called.\nDrag off pins to build functionality.
)

(event EventEnterAOE
  (params (Affected%20Pawn :type Character%20Object%20Reference))
  (if (Pawn|IsPlayerControlled Affected%20Pawn)
    (CallFunction|StartDamage Affected%20Pawn)))

(event EventExitAOE
  (params (Affected%20Pawn :type Character%20Object%20Reference))
  (if (Pawn|IsPlayerControlled Affected%20Pawn)
    (CallFunction|StopDamage)))

(fn ConstructionScript
  (|CallParentFunction))