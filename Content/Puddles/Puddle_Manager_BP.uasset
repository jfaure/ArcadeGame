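; Puddle manager that moves a character from one Teleport_Puddle_BP to another random one.
; It gathers all teleport puddles on BeginPlay, and Teleport temporarily removes the source puddle from the list while picking.
; The character is added to a picked puddle's RecentActors and moved to a picked location.
; Random is evaluated separately for each step, so those two puddles can differ.
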(event Custom|Teleport
  (params (Puddle :type Teleport%20Puddle%20BP%20Object%20Reference) (Character :type Character%20Object%20Reference))
  (bind _teleport_puddles (Variables|Default|GetTeleport%20Puddles))
  (bind (_outitem _outindex) (Utilities|Array|Random _teleport_puddles))
  (Utilities|Array|RemoveItem (Variables|Default|GetTeleport%20Puddles) Puddle)
  (if (!= _outindex -1)
    (Utilities|Array|AddUnique (Variables|/Game/Puddles/Teleport_Puddle_BP.Teleport_Puddle_BP_C|GetRecent%20Actors _outitem) Character)
    (Transformation|SetActorLocation Character (Transformation|GetActorLocation _outitem) false false))
  (Utilities|Array|AddUnique (Variables|Default|GetTeleport%20Puddles) Puddle))

(event EventBeginPlay
  (bind _outactors (Actor|GetAllActorsOfClass "/Game/Puddles/Teleport_Puddle_BP.Teleport_Puddle_BP_C"))
  (Variables|Default|SetTeleport%20Puddles _outactors))

(event Collision|EventActorBeginOverlap
  (params (OtherActor :type Actor%20Object%20Reference)))

(event EventTick
  (params (DeltaSeconds :type Float%20%28single-precision%29)))

(fn ConstructionScript)