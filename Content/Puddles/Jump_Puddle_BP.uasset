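; Jump puddle area-of-effect actor that throws pawns upward when they enter it.
; It extends a parent that supplies the EnterAOE and ExitAOE events; entering applies a large vertical force to the pawn's CharacterMovement, while exiting does nothing.
; After running the parent's BeginPlay, the puddle destroys itself following a fixed delay of several seconds.
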(event EventBeginPlay
  (|CallParentFunction)
  (Utilities|FlowControl|Delay 2e+01)
  (Actor|DestroyActor))

(event Collision|EventActorBeginOverlap
  (params (OtherActor :type Actor%20Object%20Reference))
  (|CallParentFunction OtherActor) ; This node is disabled and will not be called.\nDrag off pins to build functionality.
)

(event EventTick
  (params (DeltaSeconds :type Float%20%28single-precision%29))
  (|CallParentFunction DeltaSeconds) ; This node is disabled and will not be called.\nDrag off pins to build functionality.
)

(event EventEnterAOE
  (params (Affected%20Pawn :type Character%20Object%20Reference))
  (Physics|AddForce (Variables|/Script/Engine.Character|GetCharacterMovement Affected%20Pawn) "0, 0,4000000.000000"))

(event EventExitAOE
  (params (Affected%20Pawn :type Character%20Object%20Reference)))

(fn ConstructionScript
  (|CallParentFunction))