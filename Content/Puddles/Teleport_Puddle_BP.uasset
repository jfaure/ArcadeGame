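; Puddle actor that teleports pawns entering its area of effect, delegating the move to the level's Puddle_Manager_BP.
; It finds and caches the manager on BeginPlay, then passes itself and the entering pawn to the manager's Teleport.
; Pawns listed in RecentActors are skipped on entry and removed from that list on exit.
; Nothing in this graph adds pawns to RecentActors.
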(event EventBeginPlay
  (|CallParentFunction)
  (bind _returnvalue (Actor|GetActorOfClass "/Game/Puddles/Puddle_Manager_BP.Puddle_Manager_BP_C"))
  (Variables|Default|SetPuddle%20Manager _returnvalue))

(event Collision|EventActorBeginOverlap
  (params (OtherActor :type Actor%20Object%20Reference))
  (|CallParentFunction OtherActor) ; This node is disabled and will not be called.\nDrag off pins to build functionality.
)

(event EventTick
  (params (DeltaSeconds :type Float%20%28single-precision%29))
  (|CallParentFunction DeltaSeconds) ; This node is disabled and will not be called.\nDrag off pins to build functionality.
)

(event EventEnterAOE
  (params (Affected%20Pawn :type Character%20Object%20Reference))
  (if (not (Utilities|Array|ContainsItem (Variables|Default|GetRecent%20Actors) Affected%20Pawn))
    (Default|Teleport (Variables|Default|GetPuddle%20Manager) self Affected%20Pawn)))

(event EventExitAOE
  (params (Affected%20Pawn :type Character%20Object%20Reference))
  (Utilities|Array|RemoveItem (Variables|Default|GetRecent%20Actors) Affected%20Pawn))

(fn ConstructionScript
  (|CallParentFunction))