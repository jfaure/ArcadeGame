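; Damage cube actor that turns into a damage puddle when its SpawnPuddle event runs.
; The event spawns a Damage_Puddle_BP at the Mesh component's world location, then destroys the cube.
; Nothing in this graph calls the event, and BeginPlay, overlap and Tick are unused disabled stubs.
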(event EventBeginPlay
  (|CallParentFunction) ; This node is disabled and will not be called.\nDrag off pins to build functionality.
)

(event Collision|EventActorBeginOverlap
  (params (OtherActor :type Actor%20Object%20Reference))
  (|CallParentFunction OtherActor) ; This node is disabled and will not be called.\nDrag off pins to build functionality.
)

(event EventTick
  (params (DeltaSeconds :type Float%20%28single-precision%29))
  (|CallParentFunction DeltaSeconds) ; This node is disabled and will not be called.\nDrag off pins to build functionality.
)

(event EventSpawnPuddle
  (Game|SpawnActorfromClass "/Game/Puddles/Damage_Puddle_BP.Damage_Puddle_BP_C" (Math|Conversions|ToTransform(Vector) (Transformation|GetWorldLocation (Variables|Character|GetMesh self))) "Undefined" 0 0)
  (Actor|DestroyActor))

(fn ConstructionScript
  (|CallParentFunction))