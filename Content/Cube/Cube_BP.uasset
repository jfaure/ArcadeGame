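; Cube_BP is a cube actor with an animated skeletal mesh that handles its own death.
; OnDeath sets IsDead on the mesh's Cube_Anim_BP instance, then calls SpawnPuddle.
; SpawnPuddle is a stub that only prints a debug string, and BeginPlay, Tick and the construction script add no logic.
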(event Custom|Spawn%20Puddle
  (Development|PrintString "spawn"))

(event EventBeginPlay
  (|CallParentFunction) ; This node is disabled and will not be called.\nDrag off pins to build functionality.
)

(event EventTick
  (params (DeltaSeconds :type Float%20%28single-precision%29))
  (|CallParentFunction DeltaSeconds) ; This node is disabled and will not be called.\nDrag off pins to build functionality.
)

(event EventOnDeath
  (bind _ascube_anim_bp (Utilities|Casting|CastToCube_Anim_BP (Components|SkeletalMesh|GetAnimInstance (Variables|Character|GetMesh self))))
  (Variables|/Game/Cube/Cube_Anim_BP.Cube_Anim_BP_C|SetIs%20Dead _ascube_anim_bp true)
  (CallFunction|SpawnPuddle))

(fn ConstructionScript
  (|CallParentFunction))